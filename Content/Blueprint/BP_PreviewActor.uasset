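; BP_PreviewActor is a preview actor that shows a static mesh, apparently for previewing a spawn placement before it is confirmed.
; Its events act on the SMPreviewMesh component, swapping its mesh and collision mode from the actor's variables.
; The first material slot switches between valid and invalid materials based on IsValidSpawn, or resets to an indexed entry in a default materials array.
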(event Custom|SwitchPreviewMesh
  (Components|StaticMesh|SetStaticMesh (Variables|Default|GetSM_PreviewMesh) (Variables|Default|GetNewMesh)))

(event Custom|SwitchMaterial
  (if (Variables|Default|GetisValidSpawn)
    (Rendering|Material|SetMaterial (Variables|Default|GetSM_PreviewMesh) 0 (Variables|Default|GetvalidMaterial))
    (else
      (Rendering|Material|SetMaterial (Variables|Default|GetSM_PreviewMesh) 0 (Variables|Default|GetinvalidMaterial)))))

(event Custom|SwitchCollisionType
  (Collision|SetCollisionEnabled (Variables|Default|GetSM_PreviewMesh) (Variables|Default|GetcollisionType)))

(event Custom|SetDefaultMaterial
  (Rendering|Material|SetMaterial (Variables|Default|GetSM_PreviewMesh) 0 (Utilities|Array|Get(acopy) (Variables|Default|GetdefaultMaterials) (Variables|Default|GetdefaultMaterialIndex))))

(fn ConstructionScript)